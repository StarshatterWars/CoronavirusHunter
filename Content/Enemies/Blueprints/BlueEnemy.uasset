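; BlueEnemy is an enemy Blueprint variant that configures its star-shaped look in the Construction Script.
; It assigns a non-pulsing wireframe core material and star mesh before calling the parent script, then disables EnemyMesh collision.
; InnerStar receives the master enemy material as a dynamic instance with throb zeroed.
; EnemyColor feeds both that instance and EnemyMatInst, whose brightness is also set.
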(fn ConstructionScript
  (bind _enemymatinst (Variables|Default|GetEnemyMatInst))
  (bind _innerstar (Variables|Default|GetInnerStar))
  (Variables|Default|SetCoreMaterial "/Game/Enemies/Materials/MI_WireframeMaster_NoPulse.MI_WireframeMaster_NoPulse")
  (Variables|Default|SetEnemy%20Shape "/Game/Enemies/Meshes/SM_StarEnemy.SM_StarEnemy")
  (|CallParentFunction)
  (Collision|SetCollisionEnabled (Variables|Default|GetEnemyMesh) "NoCollision")
  (Rendering|Material|SetMaterial _innerstar 0 "/Game/Enemies/Materials/M_MasterEnemy.M_MasterEnemy")
  (bind _returnvalue (Rendering|Material|CreateDynamicMaterialInstance _innerstar 0 0 "None" :!class /Script/Engine.PrimitiveComponent))
  (Rendering|Material|SetVectorParameterValue _enemymatinst "EnemyColor" (Variables|Default|GetEnemyColor) :!class /Script/Engine.MaterialInstanceDynamic)
  (Rendering|Material|SetScalarParameterValue _returnvalue "Throb Amount" 0.0 :!class /Script/Engine.MaterialInstanceDynamic)
  (Rendering|Material|SetScalarParameterValue _enemymatinst "Brightness" 5e+01 :!class /Script/Engine.MaterialInstanceDynamic))